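; BP_GTA_R is a playable third-person-style Character Blueprint that handles movement, camera look and jumping from player input.
; Movement axes push along forward and right vectors built from control-rotation yaw only, while look axes feed controller yaw and pitch.
; Each Tick it casts the mesh's anim instance to GTA_RAnimBP and pushes horizontal speed and falling state to drive animation.
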(event `InputAction|Jump`
  (params (Key :type "Key Structure"))
  (:`Pressed`
    (`self.Jump`)))

(event `self.ReceiveTick`
  (params (DeltaSeconds :type "Float (single-precision)"))
  (bind _asgta_ranim_bp (cast `/Game/Blueprints/Review_6/GTA_RAnimBP` (`SkeletalMeshComponent.GetAnimInstance` (`self.Mesh`))))
  (set `/Game/Blueprints/Review_6/GTA_RAnimBP.이동속도_애님` (`KismetMathLibrary.VSizeXY` (`self.GetVelocity`)) _asgta_ranim_bp)
  (set `/Game/Blueprints/Review_6/GTA_RAnimBP.점프중?` (`NavMovementComponent.IsFalling` (`self.CharacterMovement`)) _asgta_ranim_bp))

(event `InputAxis|UpDown`
  (params (AxisValue :type "Float (single-precision)"))
  (bind (_returnvalue_roll _returnvalue_pitch _returnvalue_yaw) (`KismetMathLibrary.BreakRotator` (`self.GetControlRotation`)))
  (`self.AddMovementInput` (`KismetMathLibrary.GetForwardVector` (`KismetMathLibrary.MakeRotator` 0.0 0.0 _returnvalue_yaw)) AxisValue))

(event `InputAxis|LeftRight`
  (params (AxisValue :type "Float (single-precision)"))
  (bind (_returnvalue_roll _returnvalue_pitch _returnvalue_yaw) (`KismetMathLibrary.BreakRotator` (`self.GetControlRotation`)))
  (`self.AddMovementInput` (`KismetMathLibrary.GetRightVector` (`KismetMathLibrary.MakeRotator` 0.0 0.0 _returnvalue_yaw)) AxisValue))

(event `InputAxis|Turn`
  (params (AxisValue :type "Float (single-precision)"))
  ;[1 1 1] 좌우회전
  (`self.AddControllerYawInput` AxisValue))

(event `InputAxis|LookUp`
  (params (AxisValue :type "Float (single-precision)"))
  ;[1 1 1] 상하회전
  (`self.AddControllerPitchInput` AxisValue))

(fn `UserConstructionScript`)