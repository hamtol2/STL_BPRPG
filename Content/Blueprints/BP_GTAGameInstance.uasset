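; BP_GTAGameInstance is a game instance Blueprint exposing shared events for map loading, monster spawning, input mode and UI setup.
; 게임맵로드 clears all widgets and opens BlockLevelMain, while 몬스터생성 spawns BP_MonsterBear with its behavior tree at a stored location and rotation.
; 입력막기 switches input to UI-only.
; UI보이기 has BP_Controller build its UI, sets Game-and-UI input, then casts to BP_CharacterGTA without using the result.
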(event `게임맵 로드`
  (`WidgetLayoutLibrary.RemoveAllWidgets`)
  (`GameplayStatics.OpenLevel` "BlockLevelMain" false))

(event `몬스터 생성`
  (`AIBlueprintHelperLibrary.SpawnAIFromClass` "/Game/Blueprints/Monster/BP_MonsterBear.BP_MonsterBear_C" "/Game/Blueprints/Monster/AI/BT_MonsterBear.BT_MonsterBear" (`self.몬스터 생성 위치`) (`self.몬스터 생성 회전`)))

(event `입력 막기`
  (`WidgetBlueprintLibrary.SetInputMode_UIOnlyEx` (`GameplayStatics.GetPlayerController` 0) null))

(event `UI 보이기`
  (bind _asbp_controller (cast `/Game/Blueprints/Character/BP_Controller` (`GameplayStatics.GetPlayerController` 0)))
  (`/Game/Blueprints/Character/BP_Controller.UI생성 및 초기화` _asbp_controller)
  (`WidgetBlueprintLibrary.SetInputMode_GameAndUIEx` (`GameplayStatics.GetPlayerController` 0) null)
  (cast `/Game/Blueprints/Character/BP_CharacterGTA` (`GameplayStatics.GetPlayerPawn` 0)))