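; BP_Controller is a controller that owns the main HUD widget and runs the skill cooldown.
; BeginPlay calls the GTA game instance to block input, while a separate event creates UMG_Main and adds it to the viewport.
; Health and experience updates are forwarded to that widget.
; A one-shot timer ends the fixed-length cooldown, while Tick separately counts down to refresh the widget's cooldown text and percentage.
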(event `self.ReceiveBeginPlay`
  (bind _asbp_gtagame_instance (cast `/Game/Blueprints/BP_GTAGameInstance` (`GameplayStatics.GetGameInstance`)))
  (`/Game/Blueprints/BP_GTAGameInstance.입력 막기` _asbp_gtagame_instance))

(event `UI생성 및 초기화`
  (bind _returnvalue (`|CreateWidget` "/Game/UI/UMG_Main.UMG_Main_C"))
  (bind _output_get (set `self.메인UI` _returnvalue))
  (`UserWidget.AddToViewport` _output_get 0))

(event `체력 게이지 설정`
  (params (`체력 퍼센티지` :type "Float (double-precision)"))
  (`/Game/UI/UMG_Main.체력게이지 설정` (`self.메인UI`) `체력 퍼센티지`))

(event `self.ReceiveTick`
  (params (DeltaSeconds :type "Float (single-precision)"))
  (bind `_메인ui` (`self.메인UI`))
  (if (not (`self.스킬 사용 가능?`))
    (bind _output_get (set `self.쿨다운 시간` (- (`self.쿨다운 시간`) DeltaSeconds)))
    (`/Game/UI/UMG_Main.쿨다운 텍스트 설정` `_메인ui` (`KismetTextLibrary.Conv_IntToText` (`KismetMathLibrary.FTrunc` (+ _output_get 1.0))))
    (`/Game/UI/UMG_Main.쿨다운 퍼센트 설정` `_메인ui` (/ (`self.쿨다운 시간`) 10.0))))

(event `쿨다운 시작`
  (bind _returnvalue (`KismetSystemLibrary.K2_SetTimerDelegate` (delegate `쿨다운 종료`) 10.0))
  (set `self.타이머 핸들` _returnvalue)
  (set `self.스킬 사용 가능?` false)
  (set `self.쿨다운 시간` 10.0)
  (`/Game/UI/UMG_Main.쿨다운 켜기/끄기` (`self.메인UI`) true))

(event `쿨다운 종료`
  (set `self.스킬 사용 가능?` true)
  (`KismetSystemLibrary.K2_PauseTimerHandle` (`self.타이머 핸들`))
  (set `self.쿨다운 시간` 0.0)
  (`/Game/UI/UMG_Main.쿨다운 텍스트 설정` (`self.메인UI`) "")
  (`/Game/UI/UMG_Main.쿨다운 켜기/끄기` (`self.메인UI`) false))

(event `경험치 게이지 설정`
  (params (`경험치 게이지` :type "Float (double-precision)"))
  (`/Game/UI/UMG_Main.경험치 설정` (`self.메인UI`) `경험치 게이지`))

(fn `UserConstructionScript`)