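; BP_WeaponItem is a weapon pickup that a BP_CharacterGTA collects by walking into it.
; Its Item component spins around the yaw axis every Tick, scaled by delta time.
; On overlap, if the character's 무기수집가능 (can collect weapon) flag is set, it passes Item's skeletal mesh to the character's 무기수집 (collect weapon) function, then destroys itself.
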(event `self.ReceiveActorBeginOverlap`
  (params (OtherActor :type "Actor Object Reference"))
  (bind _asbp_character_gta (cast `/Game/Blueprints/Character/BP_CharacterGTA` OtherActor))
  (if (`/Game/Blueprints/Character/BP_CharacterGTA.무기수집가능?` _asbp_character_gta)
    (`/Game/Blueprints/Character/BP_CharacterGTA.무기 수집` _asbp_character_gta (`SkinnedMeshComponent.SkeletalMesh` (`self.Item`)))
    (`self.K2_DestroyActor`)))

(event `self.ReceiveTick`
  (params (DeltaSeconds :type "Float (single-precision)"))
  (`SceneComponent.K2_AddLocalRotation` (`self.Item`) (`KismetMathLibrary.MakeRotator` 0.0 0.0 (* DeltaSeconds 60.0)) false false))

(fn `UserConstructionScript`)