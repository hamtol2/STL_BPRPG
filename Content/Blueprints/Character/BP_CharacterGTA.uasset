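; Player character with axis movement, weapon pickup and drop, melee combo attacks, health and death, plus a level-restart key.
; A state enum gates movement and jumping, and Tick copies it and the armed flag to the AnimBP.
; Attacks queue montage sections for combo jumps, while externally called events toggle a hit collision that applies damage once per window.
; Damage taken flashes the mesh material via timeline and updates BP_Controller's health gauge.
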(event `Key|R`
  (params (Key :type "Key Structure"))
  ;[1 1 1] R 키 누르면 재시작
  (:`Pressed`
    (bind _returnvalue (`GameplayStatics.GetCurrentLevelName` true))
    (`GameplayStatics.OpenLevel` (`KismetStringLibrary.Conv_StringToName` _returnvalue))))

(event `self.ReceiveBeginPlay`
  (`PrimitiveComponent.SetCollisionEnabled` (`self.AttackCollision`) "NoCollision")
  (set `self.현재체력` (`self.원래체력`)))

(event `self.ReceiveTick`
  (params (DeltaSeconds :type "Float (single-precision)"))
  (bind _ascharacter_anim_bp (cast `/Game/Blueprints/Character/CharacterAnimBP` (`SkeletalMeshComponent.GetAnimInstance` (`self.Mesh`))))
  ;[1 1 1] 블루프린트 변수를 애니메이션 변수에 저장
  (set `/Game/Blueprints/Character/CharacterAnimBP.무기소유중?` (`self.무기소유중?_블프`) _ascharacter_anim_bp)
  (set `/Game/Blueprints/Character/CharacterAnimBP.캐릭터상태_애님` (`self.캐릭터상태_블프`) _ascharacter_anim_bp))

(event `InputAxis|UpDown`
  (params (AxisValue :type "Float (single-precision)"))
  (bind (_returnvalue_roll _returnvalue_pitch _returnvalue_yaw) (`KismetMathLibrary.BreakRotator` (`self.GetControlRotation`)))
  (switch `/Game/Blueprints/Character/캐릭터상태열거형` (`self.캐릭터상태_블프`)
    (:`NewEnumerator0`
      (`self.AddMovementInput` (`KismetMathLibrary.GetForwardVector` (`KismetMathLibrary.MakeRotator` 0.0 0.0 _returnvalue_yaw)) AxisValue))))

(event `InputAxis|LeftRight`
  (params (AxisValue :type "Float (single-precision)"))
  (switch `/Game/Blueprints/Character/캐릭터상태열거형` (`self.캐릭터상태_블프`)
    (:`NewEnumerator0`
      (`self.AddMovementInput` (`KismetMathLibrary.GetRightVector` (`self.GetControlRotation`)) AxisValue))))

(event `InputAxis|Turn`
  (params (AxisValue :type "Float (single-precision)"))
  (`self.AddControllerYawInput` AxisValue))

(event `InputAction|Jump`
  (params (Key :type "Key Structure"))
  (:`Pressed`
    (if (`|EnumInequality` (`self.캐릭터상태_블프`) "NewEnumerator2")
      (`self.Jump`))))

(event `InputAxis|LookUp`
  (params (AxisValue :type "Float (single-precision)"))
  (`self.AddControllerPitchInput` AxisValue))

(event `무기수집 제한하기`
  (set `self.무기수집가능?` false)
  (`KismetSystemLibrary.Delay` 2.0)
  (set `self.무기수집가능?` true))

(event `무기 수집`
  (params (`수집한 무기 메시` :type "SkeletalMesh Object Reference"))
  (if (`self.무기수집가능?`)
    (`self.무기수집 제한하기`)
    (if (`self.무기소유중?_블프`)
      (`self.무기 떨구기`))
    (`SkinnedMeshComponent.SetSkinnedAssetAndUpdate` (`self.Weapon`) `수집한 무기 메시` true)
    (set `self.무기소유중?_블프` true)
    (set `CharacterMovementComponent.MaxWalkSpeed` (`self.뛰는 속도`) (`self.CharacterMovement`))))

(event `무기 떨구기`
  (if (`self.무기소유중?_블프`)
    (set `self.무기소유중?_블프` false)
    (bind _returnvalue (`|SpawnActorFromClass` "/Game/Blueprints/Character/BP_WeaponItem.BP_WeaponItem_C" (`KismetMathLibrary.MakeTransform` (+ (`self.K2_GetActorLocation`) (* (`self.GetActorForwardVector`) 100.0))) "Undefined" "OverrideRootScale" null null))
    (`SkinnedMeshComponent.SetSkinnedAssetAndUpdate` (`/Game/Blueprints/Character/BP_WeaponItem.Item` _returnvalue) (`SkinnedMeshComponent.SkeletalMesh` (`self.Weapon`)) true)
    (`SkinnedMeshComponent.SetSkinnedAssetAndUpdate` (`self.Weapon`) null true)
    (set `CharacterMovementComponent.MaxWalkSpeed` 400.0 (`self.CharacterMovement`))))

(event `Key|X`
  (params (Key :type "Key Structure"))
  (:`Pressed`
    (`self.무기 떨구기`)))

(event `공격시작`
  (bind _returnvalue (`SkeletalMeshComponent.GetAnimInstance` (`self.Mesh`)))
  ;[1 1 1] 점프 안 할 때만 공격
  (if (`NavMovementComponent.IsFalling` (`self.CharacterMovement`))
    _
    (elif (`self.무기소유중?_블프`)
      (`self.캐릭터 상태 설정` "NewEnumerator1")
      ;[1 1 1] 몽타주가 재생 중인지 확인해서 공격 상태인지 확인
      (if (`AnimInstance.Montage_IsPlaying` _returnvalue "/Game/Characters/Animations/CharacterAnimMontage.CharacterAnimMontage")
        (switch `name` (`AnimInstance.Montage_GetCurrentSection` _returnvalue "/Game/Characters/Animations/CharacterAnimMontage.CharacterAnimMontage")
          (:`공격1`
            (set `self.다음 공격 섹션 이름` "공격2"))
          (:`공격2`
            (set `self.다음 공격 섹션 이름` "공격3"))
          (:`공격3`
            (set `self.다음 공격 섹션 이름` "공격4")))
        (else
          (`AnimInstance.Montage_Play` (`SkeletalMeshComponent.GetAnimInstance` (`self.Mesh`)) "/Game/Characters/Animations/CharacterAnimMontage.CharacterAnimMontage" 1.0 "MontageLength" 0.0 true))))))

(event `공격종료`
  (`self.캐릭터 상태 설정` "NewEnumerator0"))

(event `콤보 공격 처리`
  (bind `_다음_공격_섹션_이름` (`self.다음 공격 섹션 이름`))
  (if (!= `_다음_공격_섹션_이름` "None")
    (`AnimInstance.Montage_JumpToSection` (`SkeletalMeshComponent.GetAnimInstance` (`self.Mesh`)) `_다음_공격_섹션_이름` "/Game/Characters/Animations/CharacterAnimMontage.CharacterAnimMontage")
    (set `self.다음 공격 섹션 이름` "None")))

(event `공격판정 시작`
  (`PrimitiveComponent.SetCollisionEnabled` (`self.AttackCollision`) "QueryAndPhysics"))

(event `공격판정 종료`
  (`PrimitiveComponent.SetCollisionEnabled` (`self.AttackCollision`) "NoCollision"))

(event `self.AttackCollision.OnComponentBeginOverlap`
  (params (OverlappedComponent :type "PrimitiveComponent Object Reference") (OtherActor :type "Actor Object Reference") (OtherComp :type "PrimitiveComponent Object Reference") (OtherBodyIndex :type Integer) (bFromSweep :type Boolean) (SweepResult :type "HitResult Structure (by ref)"))
  (`GameplayStatics.ApplyDamage` OtherActor 20.0 (`self.GetController`) self)
  (`PrimitiveComponent.SetCollisionEnabled` (`self.AttackCollision`) "NoCollision"))

(event `self.ReceiveAnyDamage`
  (params (Damage :type "Float (single-precision)") (DamageType :type "DamageType Object Reference") (InstigatedBy :type "Controller Object Reference") (DamageCauser :type "Actor Object Reference"))
  (set `self.현재체력` (- (`self.현재체력`) Damage))
  (`self.대미지 색상 적용`)
  (`self.체력 게이지 업데이트`)
  (if (not (> (`self.현재체력`) 0.0))
    (`self.캐릭터 상태 설정` "NewEnumerator2")
    ;[1 1 1] 콜리전 끄기
    (`PrimitiveComponent.SetCollisionEnabled` (`self.CapsuleComponent`) "NoCollision")))

(event `캐릭터 상태 설정`
  (params (`캐릭터상태` :type "/Game/Blueprints/Character/캐릭터상태열거형 Enum" :default "NewEnumerator0"))
  (if (`|EnumInequality` (`self.캐릭터상태_블프`) "NewEnumerator2")
    (set `self.캐릭터상태_블프` `캐릭터상태`)))

(event `대미지 색상 적용`
  (bind (_direction `_대미지_색상_채널_값`) (`Timeline|대미지 색상` :!via `PlayFromStart`)
    (:`Update`
      (`MeshComponent.SetVectorParameterValueOnMaterials` (`self.Mesh`) "색상" (`KismetMathLibrary.MakeVector` 0.0 0.0 `_대미지_색상_채널_값`)))))

(event `체력 게이지 업데이트`
  (bind _asbp_controller (cast `/Game/Blueprints/Character/BP_Controller` (`GameplayStatics.GetPlayerController` 0)))
  (`/Game/Blueprints/Character/BP_Controller.체력 게이지 설정` _asbp_controller (/ (`self.현재체력`) (`self.원래체력`))))

(fn `UserConstructionScript`)