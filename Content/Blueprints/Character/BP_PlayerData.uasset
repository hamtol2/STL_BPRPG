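; BP_PlayerData holds the player's level, experience and health, with functions for an alive check and HP/EXP gauge ratios.
; Per-level stats come from a DataTable keyed by level number.
; Initialization and XP gain recompute the level by scanning rows for the first ReqEXP above current XP.
; A level-up loads the new row, refills health to MaxHP and notifies BP_CharacterGTA; damage simply subtracts from health.
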(event `레벨 확인`
  (set `self.기존레벨` (`self.현재레벨`))
  (set `self.루프인덱스` 0)
  (set `self.루프실행 여부` true)
  (`|ExecutionSequence`
    (:`then_0`
      (while (`self.루프실행 여부`)
        (bind _result (`/Engine/EditorBlueprintResources/StandardMacros.IncrementInt` (`self.루프인덱스`))
          (:`  `
            (bind `_레벨_데이터` (`self.캐릭터 레벨데이터 얻어오기` _result))
            (if (< (`self.경험치`) (`.ReqEXP_7_AAAF05A9404E27B4E017088AE9BFA1FD` (break `/Game/Blueprints/Data/SPlayerData` `_레벨_데이터`)))
              (set `self.루프실행 여부` false))))))
    (:`then_1`
      (bind _output_get (set `self.레벨인덱스` (- (`self.루프인덱스`) 1)))
      (set `self.현재레벨` _output_get)
      (if (and (!= (`self.기존레벨`) -1) (!= (`self.기존레벨`) (`self.현재레벨`)))
        (`self.레벨업`)))))

(event `초기화`
  (`self.레벨 확인`)
  (bind `_레벨_데이터` (`self.캐릭터 레벨데이터 얻어오기` (`self.현재레벨`)))
  (bind _output_get (set `self.레벨데이터` `_레벨_데이터`))
  (set `self.현재체력` (`.MaxHP_2_34F68F0149EB0190F73F5A99B7AE7663` (break `/Game/Blueprints/Data/SPlayerData` _output_get))))

(event `레벨업`
  (bind `_레벨_데이터` (`self.캐릭터 레벨데이터 얻어오기` (`self.현재레벨`)))
  (bind _output_get (set `self.레벨데이터` `_레벨_데이터`))
  (set `self.현재체력` (`.MaxHP_2_34F68F0149EB0190F73F5A99B7AE7663` (break `/Game/Blueprints/Data/SPlayerData` _output_get)))
  (bind _asbp_character_gta (cast `/Game/Blueprints/Character/BP_CharacterGTA` (`GameplayStatics.GetPlayerPawn` 0)))
  (`/Game/Blueprints/Character/BP_CharacterGTA.레벨업` _asbp_character_gta))

(event `경험치 획득`
  (params (`획득 경험치` :type Integer))
  (set `self.경험치` (+ (`self.경험치`) `획득 경험치`))
  (`self.레벨 확인`))

(event `대미지 처리`
  (params (`기본 대미지` :type "Float (double-precision)"))
  (set `self.현재체력` (- (`self.현재체력`) `기본 대미지`)))

(fn `경험치 게이지 얻어오기`
  (returns (`경험치 게이지` :type "Float (double-precision)"))
  ;[1 1 1] 다음 레벨 데이터
  (bind `_레벨_데이터` (`self.캐릭터 레벨데이터 얻어오기` (+ (`self.현재레벨`) 1)))
  (return (/ (`KismetMathLibrary.Conv_IntToDouble` (- (`self.경험치`) (`.ReqEXP_7_AAAF05A9404E27B4E017088AE9BFA1FD` (break `/Game/Blueprints/Data/SPlayerData` (`self.레벨데이터`))))) (`KismetMathLibrary.Conv_IntToDouble` (- (`.ReqEXP_7_AAAF05A9404E27B4E017088AE9BFA1FD` (break `/Game/Blueprints/Data/SPlayerData` `_레벨_데이터`)) (`.ReqEXP_7_AAAF05A9404E27B4E017088AE9BFA1FD` (break `/Game/Blueprints/Data/SPlayerData` (`self.레벨데이터`))))))))

(fn `살았나?`
  (returns (`살았나?` :type Boolean))
  (return (> (`self.현재체력`) 0.0)))

(fn `체력 게이지 얻어오기`
  (returns (`체력 게이지` :type "Float (double-precision)"))
  (return (/ (`self.현재체력`) (`.MaxHP_2_34F68F0149EB0190F73F5A99B7AE7663` (break `/Game/Blueprints/Data/SPlayerData` (`self.레벨데이터`))))))

(fn `캐릭터 레벨데이터 얻어오기`
  (params (`레벨` :type Integer))
  (returns (`레벨 데이터` :type "/Game/Blueprints/Data/SPlayerData Structure"))
  (bind _returnvalue (`|GetDataTableRow` (`self.플레이어데이터 테이블`) (`KismetStringLibrary.Conv_StringToName` (`KismetStringLibrary.Conv_IntToString` `레벨`)))
    (:`then`
      (return _returnvalue))))