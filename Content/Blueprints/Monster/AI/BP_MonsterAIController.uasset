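; AI controller for a monster that drives the possessed pawn with the bear monster behavior tree.
; On possess, it initializes the BT_MonsterBearBB blackboard with a fixed wait time and the pawn's current location as its original position.
; It then runs BT_MonsterBear; the controller has no active BeginPlay or Tick logic.
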(event `self.ReceivePossess`
  (params (PossessedPawn :type "Pawn Object Reference"))
  (`|ExecutionSequence`
    (:`then_0`
      ;[1 1 1] 초기 데이터 설정
      (`self.UseBlackboard` "/Game/Blueprints/Monster/AI/BT_MonsterBearBB.BT_MonsterBearBB")
      (`BlackboardComponent.SetValueAsFloat` (`self.Blackboard`) (`self.대기시간 키 이름`) 3.0)
      (`BlackboardComponent.SetValueAsVector` (`self.Blackboard`) (`self.원래위치 키 이름`) (`self.K2_GetActorLocation` (`self.K2_GetPawn`))))
    (:`then_1`
      (`self.RunBehaviorTree` "/Game/Blueprints/Monster/AI/BT_MonsterBear.BT_MonsterBear"))))

(fn `UserConstructionScript`)