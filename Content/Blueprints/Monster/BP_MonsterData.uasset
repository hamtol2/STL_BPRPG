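; BP_MonsterData holds a monster's level-based stats and current health.
; 레벨데이터설정 looks up the current level's row in the monster data table, caches it and fills health from MaxHP.
; 대미지처리 subtracts and returns damage from 대미지공식, which randomizes the base slightly, subtracts Defence and enforces a minimum.
; Helpers report alive state and health-bar ratio; the experience-transfer event 경험치전달 is an empty stub.
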(event `레벨데이터 설정`
  ;[1 1 1] 현재 레벨 데이터 설정하기
  (bind _returnvalue (`|GetDataTableRow` (`self.몬스터데이터 테이블`) (`KismetStringLibrary.Conv_StringToName` (`KismetStringLibrary.Conv_IntToString` (`self.현재레벨`))))
    (:`then`
      (bind _output_get (set `self.레벨데이터` _returnvalue))
      (set `self.현재체력` (`.MaxHP_2_18CF07E54AEA12F4549DBE88CF6E1FF2` (break `/Game/Blueprints/Data/SMonsterData` _output_get))))))

(event `경험치 전달`
  (params (`캐릭터 참조` :type "/Game/Blueprints/Character/BP_CharacterGTA Object Reference")))

(fn `대미지 공식`
  (params (`기본대미지` :type "Float (double-precision)"))
  (returns (`최종대미지` :type "Float (double-precision)"))
  (return (`KismetMathLibrary.FMax` (- (`KismetMathLibrary.RandomFloatInRange` (* `기본대미지` 0.9) (* `기본대미지` 1.1)) (`.Defence_10_5BB8180140637CD659AA5AACB2094E9D` (break `/Game/Blueprints/Data/SMonsterData` (`self.레벨데이터`)))) 3.0)))

(fn `대미지처리`
  (params (`기본대미지` :type "Float (double-precision)"))
  (returns (`최종대미지` :type "Float (double-precision)"))
  (bind `_최종대미지` (`self.대미지 공식` `기본대미지`))
  (set `self.현재체력` (- (`self.현재체력`) `_최종대미지`))
  (return `_최종대미지`))

(fn `살았나?`
  (returns (`살았나?` :type Boolean))
  (return (> (`self.현재체력`) 0.0)))

(fn `체력게이지 얻어오기`
  (returns (`체력게이지` :type "Float (double-precision)"))
  (return (/ (`self.현재체력`) (`.MaxHP_2_18CF07E54AEA12F4549DBE88CF6E1FF2` (break `/Game/Blueprints/Data/SMonsterData` (`self.레벨데이터`))))))