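; Bear monster enemy that spots, chases and attacks the player, and grants experience on death.
; A state enum (idle, chase, attack, dead) sets walk speed and feeds the AI blackboard and AnimBP, with PawnSensing triggering chase.
; BPMonsterData supplies level stats and damage handling, driving HUD health, damage text, hit tint and death dissolve.
; A hit flag, cleared by the player's attack-end dispatcher, blocks repeat damage within one attack.
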(event `기본 동작`
  (bind _attackcollision (`self.AttackCollision`))
  ;[1 1 1] 기본 동작 로직
  (if (`PrimitiveComponent.K2_IsCollisionEnabled` _attackcollision)
    (`PrimitiveComponent.SetCollisionEnabled` _attackcollision "NoCollision")))

(event `쫒아가기 동작`
  ;[1 1 1] 쫒아가기 동작 로직
  (if (> (`KismetMathLibrary.Vector_Distance2D` (`self.K2_GetActorLocation`) (`self.K2_GetActorLocation` (`GameplayStatics.GetPlayerPawn` 0))) (`PawnSensingComponent.SightRadius` (`self.PawnSensing`)))
    (`self.몬스터 상태 설정` "NewEnumerator0")))

(event `공격 동작`
  (bind _instigator (`self.Instigator`))
  (`/Engine/EditorBlueprintResources/StandardMacros.IsValid` _instigator
    (:`Is Valid`
      (bind _asbp_character_gta (cast `/Game/Blueprints/Character/BP_CharacterGTA` _instigator))
      (if (`|EnumEquality` (`/Game/Blueprints/Character/BP_CharacterGTA.캐릭터상태_블프` _asbp_character_gta) "NewEnumerator2")
        (`self.몬스터 상태 설정` "NewEnumerator0")))))

(event `self.ReceiveBeginPlay`
  (bind _bp_monsterdata (`self.BP_MonsterData`))
  (bind _pawnsensing (`self.PawnSensing`))
  (bind (_maxhp _attack _sightrange _sightangle) (break `/Game/Blueprints/Data/SMonsterData` (`/Game/Blueprints/Monster/BP_MonsterData.레벨데이터` _bp_monsterdata)))
  (`|ExecutionSequence`
    (:`then_0`
      (`PrimitiveComponent.SetCollisionEnabled` (`self.AttackCollision`) "NoCollision")
      (bind _asumg_hudhp (cast `/Game/UI/UMG_HUDHP` (`WidgetComponent.GetUserWidgetObject` (`self.HUDHP`))))
      (set `self.HUD위젯` _asumg_hudhp))
    (:`then_1`
      (bind _asbp_character_gta (cast `/Game/Blueprints/Character/BP_CharacterGTA` (`GameplayStatics.GetPlayerPawn` 0)))
      (set `self.캐릭터 참조` _asbp_character_gta))
    (:`then_2`
      (`/Game/Blueprints/Monster/BP_MonsterData.레벨데이터 설정` _bp_monsterdata)
      (set `PawnSensingComponent.SightRadius` _sightrange _pawnsensing)
      (`PawnSensingComponent.SetPeripheralVisionAngle` _pawnsensing _sightangle)
      (add `/Game/Blueprints/Character/BP_CharacterGTA.공격종료 디스패처` (`self.캐릭터 참조`) (delegate `맞았나 값 초기화`)))))

(event `쳐다보기`
  ;[1 1 1] 공격 당했을 때 캐릭터 쳐다보기
  (if (not (`|EnumEquality` (`self.몬스터상태_블프`) "NewEnumerator2"))
    (`self.K2_SetActorRotation` (`KismetMathLibrary.FindLookAtRotation` (`self.K2_GetActorLocation`) (`self.K2_GetActorLocation` (`GameplayStatics.GetPlayerPawn` 0))))
    (`self.몬스터 상태 설정` "NewEnumerator2")))

(event `맞았나 값 초기화`
  (set `self.맞았나?` false))

(event `self.ReceiveTick`
  (params (DeltaSeconds :type "Float (single-precision)"))
  (bind `_몬스터상태_블프` (`self.몬스터상태_블프`))
  (bind _asbear_anim_bp (cast `/Game/Blueprints/Monster/BearAnimBP` (`SkeletalMeshComponent.GetAnimInstance` (`self.Mesh`))))
  (set `/Game/Blueprints/Monster/BearAnimBP.이동속도_애님` (`KismetMathLibrary.VSize` (`self.GetVelocity`)) _asbear_anim_bp)
  (set `/Game/Blueprints/Monster/BearAnimBP.몬스터상태_애님` `_몬스터상태_블프` _asbear_anim_bp)
  (switch `/Game/Blueprints/Monster/몬스터상태_열거형` `_몬스터상태_블프`
    (:`NewEnumerator0`
      (`self.기본 동작`))
    (:`NewEnumerator2`
      (`self.쫒아가기 동작`))
    (:`NewEnumerator3`
      (`self.공격 동작`))))

(event `self.ReceiveAnyDamage`
  (params (Damage :type "Float (single-precision)") (DamageType :type "DamageType Object Reference") (InstigatedBy :type "Controller Object Reference") (DamageCauser :type "Actor Object Reference"))
  (if (not (`self.맞았나?`))
    (set `self.맞았나?` true)
    (bind `_최종대미지` (`/Game/Blueprints/Monster/BP_MonsterData.대미지처리` (`self.BP_MonsterData`) Damage))
    (`self.대미지 텍스트 애니메이션 재생` (`KismetMathLibrary.FTrunc` `_최종대미지`))
    (`self.체력 게이지 설정`)
    (`self.대미지 색상 적용`)
    ;[1 1 1] 카메라 흔들기
    (`PlayerController.ClientStartCameraShake` :`self` (`GameplayStatics.GetPlayerController` 0) :`Shake` "/Game/Blueprints/Character/BP_DamageShake.BP_DamageShake_C")
    (bind `_살았나_` (`/Game/Blueprints/Monster/BP_MonsterData.살았나?` (`self.BP_MonsterData`)))
    (if `_살았나_`
      (`self.쳐다보기`)
      (else
        ;[1 1 1] 죽는 상태로 변경
        (`self.몬스터 상태 설정` "NewEnumerator1")
        ;[1 1 1] 캐릭터에 경험치 전달
        (`/Game/Blueprints/Monster/BP_MonsterData.경험치 전달` (`self.BP_MonsterData`) (`self.캐릭터 참조`))
        ;[1 1 1] 콜리전 끄고, 5초 있다가 삭제
        (`SceneComponent.SetVisibility` (`self.HUDHP`) false false)
        (`PrimitiveComponent.SetCollisionEnabled` (`self.CapsuleComponent`) "NoCollision")
        (`self.디졸브 효과 재생`)
        (`KismetSystemLibrary.Delay` 5.0)
        (`self.K2_DestroyActor`)))))

(event `몬스터 상태 설정`
  (params (`몬스터상태` :type "/Game/Blueprints/Monster/몬스터상태_열거형 Enum" :default "NewEnumerator0"))
  (bind _charactermovement (`self.CharacterMovement`))
  (bind (_maxhp _attack _sightrange _sightangle _defence _gainexp _walkspeed _patrolwaittime _runspeed) (break `/Game/Blueprints/Data/SMonsterData` (`/Game/Blueprints/Monster/BP_MonsterData.레벨데이터` (`self.BP_MonsterData`))))
  ;[1 1 1] 죽었는지 확인
  (if (`|EnumInequality` (`self.몬스터상태_블프`) "NewEnumerator1")
    (bind _output_get (set `self.몬스터상태_블프` `몬스터상태`))
    (`|ExecutionSequence`
      (:`then_0`
        (switch `/Game/Blueprints/Monster/몬스터상태_열거형` (`self.몬스터상태_블프`)
          (:`NewEnumerator0`
            (set `CharacterMovementComponent.MaxWalkSpeed` _walkspeed _charactermovement))
          (:`NewEnumerator2`
            (set `CharacterMovementComponent.MaxWalkSpeed` _runspeed _charactermovement))
          (:`NewEnumerator3`
            (set `CharacterMovementComponent.MaxWalkSpeed` 0.0 _charactermovement :!label _label))
          (:`NewEnumerator1`
            (goto _label))))
      (:`then_1`
        (`BlackboardComponent.SetValueAsEnum` (`AIBlueprintHelperLibrary.GetBlackboard` (`self.GetController`)) (`self.몬스터상태 키 이름`) _output_get)))))

(event `체력 게이지 설정`
  ;[1 1 1] HUD에 체력 게이지 설정
  (bind `_체력게이지` (`/Game/Blueprints/Monster/BP_MonsterData.체력게이지 얻어오기` (`self.BP_MonsterData`)))
  (`/Game/UI/UMG_HUDHP.체력게이지  설정` (`self.HUD위젯`) `_체력게이지`))

(event `대미지 색상 적용`
  (bind (_direction `_대미지_색상_채널_값`) (`Timeline|대미지 색상` :!via `PlayFromStart`)
    (:`Update`
      (`MeshComponent.SetVectorParameterValueOnMaterials` (`self.Mesh`) "색상" (`KismetMathLibrary.MakeVector` `_대미지_색상_채널_값`)))))

(event `대미지 텍스트 애니메이션 재생`
  (params (`대미지` :type Integer))
  ;[1 1 1] 대미지 텍스트 애님 재생
  (`/Game/UI/UMG_HUDHP.대미지 텍스트 애니메이션 재생` (`self.HUD위젯`) `대미지`))

(event `디졸브 효과 재생`
  (bind (_direction `_디졸브_값`) (`Timeline|디졸브` :!via `PlayFromStart`)
    (:`Update`
      (`MeshComponent.SetScalarParameterValueOnMaterials` (`self.Mesh`) "디졸브" `_디졸브_값`))))

(event `self.PawnSensing.OnSeePawn`
  (params (Pawn :type "Pawn Object Reference"))
  (bind _asbp_character_gta (cast `/Game/Blueprints/Character/BP_CharacterGTA` Pawn))
  (if (`|EnumEquality` (`/Game/Blueprints/Character/BP_CharacterGTA.캐릭터상태_블프` _asbp_character_gta) "NewEnumerator2")
    _
    (elif (`|EnumInequality` (`self.몬스터상태_블프`) "NewEnumerator1")
      (bind _output_get (set `self.Instigator` _asbp_character_gta))
      (`BlackboardComponent.SetValueAsObject` (`AIBlueprintHelperLibrary.GetBlackboard` (`self.GetController`)) (`self.타겟플레이어 키 이름`) _output_get)
      (`self.몬스터 상태 설정` "NewEnumerator2"))))

(event `공격 판정 시작`
  (`PrimitiveComponent.SetCollisionEnabled` (`self.AttackCollision`) "QueryOnly"))

(event `공격 판정 종료`
  (`PrimitiveComponent.SetCollisionEnabled` (`self.AttackCollision`) "NoCollision"))

(event `self.AttackCollision.OnComponentBeginOverlap`
  (params (OverlappedComponent :type "PrimitiveComponent Object Reference") (OtherActor :type "Actor Object Reference") (OtherComp :type "PrimitiveComponent Object Reference") (OtherBodyIndex :type Integer) (bFromSweep :type Boolean) (SweepResult :type "HitResult Structure (by ref)"))
  (`GameplayStatics.ApplyDamage` OtherActor (`.Attack_4_DEFF91894C47E61BCB97B38535C3C6D9` (break `/Game/Blueprints/Data/SMonsterData` (`/Game/Blueprints/Monster/BP_MonsterData.레벨데이터` (`self.BP_MonsterData`)))) (`self.GetController`) self))

(fn `UserConstructionScript`)